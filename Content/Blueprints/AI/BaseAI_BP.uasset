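; Base enemy AI character whose stats, looks and melee or ranged behavior come from EnemyTypeDataAsset.
; It roams randomly until damage or a line-of-sight-checked vision cone triggers chasing, which also alerts nearby AI.
; It pursues the nearest player (farthest if that one is dead), attacks in range, then repositions, using paired SERVER/CLIENT events.
; Death spawns an impulse-driven gib actor, plus a key if it is a KeyHolder, which displays an animated key.
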(event `self.ReceiveBeginPlay`
  (bind _enemytype_dataasset (`self.EnemyType_DataAsset`))
  (bind _hatmesh (`self.HatMesh`))
  (bind _basematerial (`/Game/Blueprints/AI/Enemy_DA.BaseMaterial` _enemytype_dataasset))
  ; beginplay
  (`|ExecutionSequence`
    (:`then_0`
      (switch `/Game/Blueprints/AI/EnemyStates_Enum` (`self.EnemyState`)
        (:`NewEnumerator2`
          _)
        (:`NewEnumerator3`
          _))
      (`self.SERVER_RandomRoam`))
    (:`then_1`
      (bind _asbp_game_instance (cast `/Game/Blueprints/OnlineSystem/BP_GameInstance` (`GameplayStatics.GetGameInstance`)))
      (set `self.GameInstance` _asbp_game_instance))
    (:`then_2`
      (set `self.EnemyHealth` (`/Game/Blueprints/AI/Enemy_DA.Health` (`self.EnemyType_DataAsset`)))
      (set `CharacterMovementComponent.MaxWalkSpeed` (`/Game/Blueprints/AI/Enemy_DA.MovementSpeed` (`self.EnemyType_DataAsset`)) (`self.CharacterMovement`))
      (set `self.BulletsLeft` (`/Game/Blueprints/AI/Enemy_DA.Bullets` _enemytype_dataasset))
      (`StaticMeshComponent.SetStaticMesh` (`self.WeaponMesh`) (`/Game/Blueprints/AI/Enemy_DA.WeaponMesh` _enemytype_dataasset))
      (`StaticMeshComponent.SetStaticMesh` _hatmesh (`/Game/Blueprints/AI/Enemy_DA.HatMesh` _enemytype_dataasset))
      (`PrimitiveComponent.SetMaterial` (`self.Mesh`) 1 _basematerial)
      (`PrimitiveComponent.SetMaterial` _hatmesh 0 _basematerial))
    (:`then_3`
      (if (`self.KeyHolder`)
        (`SceneComponent.SetHiddenInGame` (`self.KeyMesh`) false false)
        (`|ExecutionSequence`
          (:`then_0`
            (bind (_direction _newtrack_0) (`Timeline|Timeline` :!via `PlayFromStart` :!label _label)
              (:`Update`
                (`SceneComponent.K2_SetRelativeLocation` (`self.KeyMover`) (`KismetMathLibrary.VLerp` (0.0 0.0 0.0) (0.0 0.0 25.0) _newtrack_0) false false))
              (:`Finished`
                (`|ExecutionSequence`
                  (:`then_0`
                    (goto _label :!via `PlayFromStart`))))))
          (:`then_1`
            (bind (_direction_2 _newtrack_0_2) (`Timeline|Timeline_0` :!via `PlayFromStart` :!label _label_2)
              (:`Update`
                (`SceneComponent.K2_SetRelativeRotation` (`self.KeyMover`) (`KismetMathLibrary.RLerp` (struct) (struct :`Yaw` 360.0) _newtrack_0_2) false false))
              (:`Finished`
                (`|ExecutionSequence`
                  (:`then_0`
                    (goto _label_2 :!via `PlayFromStart`)))))))))))

(event `SERVER_RandomRoam`
  ; Random Roam
  (`self.CLIENT_RandomRoam`))

(event `CLIENT_RandomRoam`
  (bind _timebetweenrandomroam (`/Game/Blueprints/AI/Enemy_DA.TimeBetweenRandomRoam` (`self.EnemyType_DataAsset`)))
  ; Random Roam
  (`|AIMoveTo` self (`NavigationSystemV1.K2_GetRandomReachablePointInRadius` (`self.K2_GetActorLocation`) (`/Game/Blueprints/AI/Enemy_DA.RandomRoamRadius` (`self.EnemyType_DataAsset`)) null null) null 25.0
    (:`OnSuccess`
      _)
    (:`OnFail`
      _))
  (`KismetSystemLibrary.Delay` (`KismetMathLibrary.RandomFloatInRange` _timebetweenrandomroam (+ _timebetweenrandomroam _timebetweenrandomroam)))
  (if (`|EnumEquality` (`self.EnemyState`) "NewEnumerator2")
    (`self.SERVER_RandomRoam`)))

(event `SERVER_ChasePlayer`
  ; Chase
  (`self.CLIENT_ChasePlayer`))

(event `CLIENT_ChasePlayer`
  (bind _aliveplayers (`/Game/Blueprints/OnlineSystem/BP_GameInstance.AlivePlayers` (`self.GameInstance`)))
  (bind _output (`|GetArrayItem` (`/Game/Blueprints/OnlineSystem/BP_GameInstance.AlivePlayers` (`self.GameInstance`)) (`KismetMathLibrary.MaxOfFloatArray` (`self.DistanceToPlayerArray`))))
  (bind _output_2 (`|GetArrayItem` _aliveplayers (`KismetMathLibrary.MinOfFloatArray` (`self.DistanceToPlayerArray`))))
  ; Chase
  (`KismetArrayLibrary.Array_Clear` (`self.DistanceToPlayerArray`))
  (for _array_element _aliveplayers
    (`KismetArrayLibrary.Array_Add` (`self.DistanceToPlayerArray`) (`KismetMathLibrary.Vector_Distance` (`self.K2_GetActorLocation` _array_element) (`self.K2_GetActorLocation`))))
  (`/Engine/EditorBlueprintResources/StandardMacros.IsValid` _output_2
    (:`Is Valid`
      (if (`self.ActorHasTag` _output_2 "dead")
        (`/Engine/EditorBlueprintResources/StandardMacros.IsValid` _output
          (:`Is Valid`
            (set `self.PlayerToChase` _output)))
        (else
          (set `self.PlayerToChase` _output_2)))
      (`|AIMoveTo` self (`NavigationSystemV1.K2_GetRandomReachablePointInRadius` (`self.K2_GetActorLocation` (`self.PlayerToChase`)) 25.0 null null) null 25.0
        (:`then`
          (`KismetSystemLibrary.DelayUntilNextTick`)
          (if (<= (`KismetMathLibrary.Vector_Distance` (`self.K2_GetActorLocation`) (`self.K2_GetActorLocation` (`self.PlayerToChase`))) (`/Game/Blueprints/AI/Enemy_DA.AttackRange` (`self.EnemyType_DataAsset`)))
            (`self.SERVER_Attack`)
            (else
              (`self.SERVER_ChasePlayer`))))))))

(event `SERVER_Reposition`
  ; Reposition
  (`self.CLIENT_Reposition`))

(event `CLIENT_Reposition`
  (bind _enemytype_dataasset (`self.EnemyType_DataAsset`))
  ; Reposition
  (`MovementComponent.StopMovementImmediately` (`self.CharacterMovement`))
  (if (`/Game/Blueprints/AI/Enemy_DA.Melee` _enemytype_dataasset)
    (set `self.MeleeRepositionMod` 2.0)
    (else
      (set `self.MeleeRepositionMod` 1.0)))
  (`|AIMoveTo` self (`NavigationSystemV1.K2_GetRandomReachablePointInRadius` (`self.K2_GetActorLocation` (`self.PlayerToChase`)) (/ (`/Game/Blueprints/AI/Enemy_DA.RandomRoamRadius` _enemytype_dataasset) (`self.MeleeRepositionMod`)) null null) null 25.0
    (:`OnSuccess`
      _)
    (:`OnFail`
      _))
  (`self.SERVER_ChasePlayer`))

(event `self.VisionCone.OnComponentBeginOverlap`
  (params (OverlappedComponent :type "PrimitiveComponent Object Reference") (OtherActor :type "Actor Object Reference") (OtherComp :type "PrimitiveComponent Object Reference") (OtherBodyIndex :type Integer) (bFromSweep :type Boolean) (SweepResult :type "HitResult Structure (by ref)"))
  ; Sight
  (if (== (`GameplayStatics.GetObjectClass` OtherActor) "/Game/Blueprints/BP_ThirdPersonCharacter.BP_ThirdPersonCharacter_C")
    (bind (_outhit _returnvalue) (`KismetSystemLibrary.LineTraceSingle` (`SceneComponent.K2_GetComponentLocation` (`self.VisionCone`)) (+ (`self.K2_GetActorLocation` OtherActor) (0.0 0.0 50.0)) "TraceTypeQuery1"))
    (if _returnvalue
      (if (== (`.HitActor` (`GameplayStatics.BreakHitResult` _outhit)) OtherActor)
        (`self.SERVER_PlayerSpotted`)))))

(event `SERVER_PlayerSpotted`
  ; Sight
  (`self.CLIENT_PlayerSpotted`)
  (`PrimitiveComponent.SetCollisionEnabled` (`self.VisionCone`) "NoCollision"))

(event `CLIENT_PlayerSpotted`
  ; Sight
  (`MovementComponent.StopMovementImmediately` (`self.CharacterMovement`))
  (set `self.EnemyState` "NewEnumerator3")
  (`KismetArrayLibrary.Array_Add` (`self.Tags`) "chasing")
  (`self.SERVER_ChasePlayer`)
  (`KismetSystemLibrary.PrintString` "PLAYER SPOTTED")
  (bind (_outactors _returnvalue) (`KismetSystemLibrary.SphereOverlapActors` (`self.K2_GetActorLocation`) (`/Game/Blueprints/AI/Enemy_DA.AwarenessSphereRadius` (`self.EnemyType_DataAsset`)) (`|MakeArray` "ObjectTypeQuery3" :!type "EObjectTypeQuery Enum") "BaseAI_BP_C" (`|MakeArray` self :!type "Actor Object Reference")))
  (if _returnvalue
    (for _array_element _outactors
      (if (not (`self.ActorHasTag` _array_element "chasing"))
        (bind _asbase_ai_bp (cast `/Game/Blueprints/AI/BaseAI_BP` _array_element))
        (`self.SERVER_PlayerSpotted` _asbase_ai_bp)))))

(event `SERVER_Attack`
  ; Attack
  (`self.CLIENT_Attack`))

(event `CLIENT_Attack`
  (bind _returnvalue (`self.K2_GetActorLocation`))
  (bind _playertochase (`self.PlayerToChase`))
  (bind _enemytype_dataasset (`self.EnemyType_DataAsset`))
  (bind _bulletsleft (`self.BulletsLeft`))
  (bind _enemytype_dataasset_2 (`self.EnemyType_DataAsset`))
  ; Attack
  (if (`/Game/Blueprints/AI/Enemy_DA.Melee` (`self.EnemyType_DataAsset`))
    (`GameplayStatics.ApplyPointDamage` _playertochase 1.0 (`KismetMathLibrary.GetDirectionUnitVector` (`self.K2_GetActorLocation` _playertochase) _returnvalue) (`GameplayStatics.MakeHitResult` false false 0.0 0.0 _returnvalue) null self)
    (`|PlayMontage` (`self.Mesh`) (`/Game/Blueprints/AI/Enemy_DA.FiringAnim` _enemytype_dataasset_2)
      (:`then`
        (`self.SERVER_Reposition` :!label _label_3)))
    (else
      (set `self.Aiming` true)
      (set `CharacterMovementComponent.MaxWalkSpeed` 0.0 (`self.CharacterMovement`))
      (`|PlayMontage` (`self.Mesh`) (`/Game/Blueprints/AI/Enemy_DA.AimAnim` _enemytype_dataasset)
        (:`then`
          (`|ExecutionSequence`
            (:`then_0`
              (`KismetSystemLibrary.Delay` (`/Game/Blueprints/AI/Enemy_DA.AimingTime` (`self.EnemyType_DataAsset`)))
              (`|PlayMontage` (`self.Mesh`) (`/Game/Blueprints/AI/Enemy_DA.FiringAnim` _enemytype_dataasset) :!label _label_4
                (:`then`
                  (`self.SERVER_FireProjectile` (`KismetMathLibrary.MakeTransform` (`SceneComponent.K2_GetComponentLocation` (`self.BulletSpawnLoc`)) (`KismetMathLibrary.Conv_VectorToRotator` (`KismetMathLibrary.GetDirectionUnitVector` (`SceneComponent.K2_GetComponentLocation` (`self.BulletSpawnLoc`)) (`self.K2_GetActorLocation` (`self.PlayerToChase`))))) "/Game/Blueprints/BaseProjectile_BP.BaseProjectile_BP_C")
                  (`/Engine/EditorBlueprintResources/StandardMacros.DecrementInt` _bulletsleft
                    (:`  `
                      (if (<= _bulletsleft 0)
                        (`KismetSystemLibrary.Delay` 0.5)
                        (set `self.Aiming` false)
                        (set `CharacterMovementComponent.MaxWalkSpeed` (`/Game/Blueprints/AI/Enemy_DA.MovementSpeed` (`self.EnemyType_DataAsset`)) (`self.CharacterMovement`))
                        (set `self.BulletsLeft` (`/Game/Blueprints/AI/Enemy_DA.Bullets` (`self.EnemyType_DataAsset`)))
                        (set `CharacterMovementComponent.RotationRate` (struct :`Yaw` 360.0) (`self.CharacterMovement`))
                        (goto _label_3)
                        (else
                          (`KismetSystemLibrary.Delay` (`/Game/Blueprints/AI/Enemy_DA.FiringSpeed` _enemytype_dataasset_2))
                          (goto _label_4))))))))
            (:`then_1`
              (`self.SERVER_Rotate`))))))))

(event `SERVER_Rotate`
  (bind (_returnvalue_roll _returnvalue_pitch) (`KismetMathLibrary.BreakRotator` (`self.K2_GetActorRotation`)))
  (bind (_returnvalue_roll_2 _returnvalue_pitch_2 _returnvalue_yaw) (`KismetMathLibrary.BreakRotator` (`KismetMathLibrary.MakeRotFromX` (`KismetMathLibrary.GetDirectionUnitVector` (`SceneComponent.K2_GetComponentLocation` (`self.BulletSpawnLoc`)) (`self.K2_GetActorLocation` (`self.PlayerToChase`))))))
  ; Attack
  (`MovementComponent.StopMovementImmediately` (`self.CharacterMovement`))
  (if (`self.Aiming`) :!label _label_5
    (`self.K2_SetActorRotation` (`KismetMathLibrary.MakeRotator` _returnvalue_roll _returnvalue_pitch _returnvalue_yaw))
    (`KismetSystemLibrary.DelayUntilNextTick`)
    (goto _label_5)))

(event `SERVER_FireProjectile`
  (params (SpawnTransform :type "Transform Structure") (Class :type "Actor Class Reference"))
  ; Attack
  (`|SpawnActorFromClass` Class SpawnTransform "AlwaysSpawn" "MultiplyWithRoot" null null)
  (`NiagaraFunctionLibrary.SpawnSystemAtLocation` "/Game/VFX/NS_WeaponFire_ShellEject.NS_WeaponFire_ShellEject" (.location SpawnTransform)))

(event `CLIENT_TakeDamage`
  (params (B :type "Float (double-precision)") (BoneName :type Name) (A :type "Vector Structure"))
  (bind _hatmesh (`self.HatMesh`))
  (bind _mesh (`self.Mesh`))
  ; Take damage
  (`|ExecutionSequence`
    (:`then_0`
      (bind _output_get (set `self.EnemyHealth` (`KismetMathLibrary.FClamp` (- (`self.EnemyHealth`) B) 0.0 999999.0)))
      (if (<= _output_get 0.0)
        (`/Engine/EditorBlueprintResources/StandardMacros.DoOnce` false
          (:`Completed`
            (if (`self.KeyHolder`)
              (`|SpawnActorFromClass` "/Game/Blueprints/CoOp/Key_Actor.Key_Actor_C" (`KismetMathLibrary.MakeTransform` (`self.K2_GetActorLocation`)) "AlwaysSpawn" "MultiplyWithRoot" null null))
            (bind _returnvalue (`|SpawnActorFromClass` "/Game/Blueprints/AI/AI_Gib_Actor.AI_Gib_Actor_C" (`self.GetTransform`) "AlwaysSpawn" "MultiplyWithRoot" null null))
            (bind _skeletalmesh (`/Game/Blueprints/AI/AI_Gib_Actor.SkeletalMesh` _returnvalue))
            (`PrimitiveComponent.AddImpulse` _skeletalmesh (* A B 12000.0) BoneName true)
            (`StaticMeshComponent.SetStaticMesh` (`/Game/Blueprints/AI/AI_Gib_Actor.HatMesh` _returnvalue) (`StaticMeshComponent.StaticMesh` _hatmesh))
            (`PrimitiveComponent.SetMaterial` _skeletalmesh 1 (`PrimitiveComponent.GetMaterial` (`self.Mesh`) 1))
            (`PrimitiveComponent.SetMaterial` _hatmesh 0 (`PrimitiveComponent.GetMaterial` (`self.HatMesh`) 0))
            (`PrimitiveComponent.SetMaterial` (`/Game/Blueprints/AI/AI_Gib_Actor.HatMesh` _returnvalue) 0 (`PrimitiveComponent.GetMaterial` (`self.HatMesh`) 0))
            (if (== (`self.EnemyType_DataAsset`) "/Game/Blueprints/AI/MachineGun_DA.MachineGun_DA")
              (`SkeletalMeshComponent.PlayAnimation` _skeletalmesh "/Game/Models/Animated/EnemyGuard/Rifle_Idle__4_.Rifle_Idle__4_" false))
            (`KismetSystemLibrary.DelayUntilNextTick`)
            (`self.K2_DestroyActor`)))
        (else
          (`PrimitiveComponent.SetMaterial` _mesh 0 "/Game/CustomMaterials/RedPlastic.RedPlastic")
          (`KismetSystemLibrary.Delay` 0.2)
          (`PrimitiveComponent.SetMaterial` _mesh 0 "/Game/CustomMaterials/Textures/skin_texture_Mat.skin_texture_Mat"))))
    (:`then_1`
      (if (not (`KismetArrayLibrary.Array_Contains` (`self.Tags`) "chasing"))
        (`/Engine/EditorBlueprintResources/StandardMacros.DoOnce` false
          (:`Completed`
            (`self.SERVER_PlayerSpotted`)))))))

(event `self.ReceivePointDamage`
  (params (Damage :type "Float (single-precision)") (DamageType :type "DamageType Object Reference") (HitLocation :type "Vector Structure") (HitNormal :type "Vector Structure") (HitComponent :type "PrimitiveComponent Object Reference") (BoneName :type Name) (ShotFromDirection :type "Vector Structure") (InstigatedBy :type "Controller Object Reference") (DamageCauser :type "Actor Object Reference") (HitInfo :type "HitResult Structure (by ref)"))
  ; Take damage
  (`self.SERVER_TakeDamage` Damage BoneName ShotFromDirection))

(event `SERVER_TakeDamage`
  (params (B :type "Float (double-precision)") (BoneName :type Name) (A :type "Vector Structure"))
  ; Take damage
  (`self.CLIENT_TakeDamage` B BoneName A))

(fn `UserConstructionScript`)