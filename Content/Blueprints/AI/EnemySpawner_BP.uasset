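; Enemy spawner actor that spawns a BaseAI_BP enemy configured by an enemy type data asset.
; Activate calls a server-named spawn event, which destroys any previous enemy, spawns a new one just above the spawner and stores it.
; The spawner passes its enemy state, data asset and key holder setting to the spawned AI.
; The construction script previews the setup with the type's name and material, showing a key mesh for key holders.
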(event `/Game/Blueprints/CoOp/CoOp_BPI.activate`
  (`self.SERVER_SpawnEnemy` (`/Game/Blueprints/AI/Enemy_DA.Name` (`self.EnemyType_DataAsset`)) (`self.Enemy State`) (`self.KeyHolder`) (`self.EnemyType_DataAsset`)))

(event `SERVER_SpawnEnemy`
  (params (Selection :type String) (EnemyState :type "/Game/Blueprints/AI/EnemyStates_Enum Enum" :default "NewEnumerator0") (KeyHolder :type Boolean) (EnemyType_DataAsset :type "/Game/Blueprints/AI/Enemy_DA Object Reference"))
  (bind _spawnedenemy (`self.SpawnedEnemy`))
  (`/Engine/EditorBlueprintResources/StandardMacros.IsValid` _spawnedenemy
    (:`Is Valid`
      (`self.K2_DestroyActor` _spawnedenemy))
    (:`Is Not Valid`
      _))
  (bind _returnvalue (`|SpawnActorFromClass` "/Game/Blueprints/AI/BaseAI_BP.BaseAI_BP_C" (`KismetMathLibrary.MakeTransform` (+ (`self.K2_GetActorLocation`) (0.0 0.0 100.0)) (`self.K2_GetActorRotation`)) "AlwaysSpawn" "MultiplyWithRoot" null EnemyState EnemyType_DataAsset KeyHolder null))
  (set `self.SpawnedEnemy` _returnvalue))

(fn `UserConstructionScript`
  (bind _enemytype_dataasset (`self.EnemyType_DataAsset`))
  (`TextRenderComponent.K2_SetText` (`self.TextRender`) (`KismetTextLibrary.Conv_StringToText` (`/Game/Blueprints/AI/Enemy_DA.Name` _enemytype_dataasset)))
  (`PrimitiveComponent.SetMaterial` (`self.Cylinder`) 0 (`/Game/Blueprints/AI/Enemy_DA.BaseMaterial` _enemytype_dataasset))
  (if (`self.KeyHolder`)
    (`SceneComponent.SetVisibility` (`self.KeyMesh`) true false)))