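; Base projectile that deals point damage and plays impact effects when it hits something.
; The first hit, gated by DoOnce, passes hit details and damage settings through a server-named event to a client-named event.
; That client event spawns a meat-impact particle, plays a sound and applies the damage, rather than the server event.
; It then disables sphere collision, hides the bullet mesh and destroys the actor after a short delay.
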(event `self.ReceiveHit`
  (params (MyComp :type "PrimitiveComponent Object Reference") (Other :type "Actor Object Reference") (OtherComp :type "PrimitiveComponent Object Reference") (bSelfMoved :type Boolean) (HitLocation :type "Vector Structure") (HitNormal :type "Vector Structure") (NormalImpulse :type "Vector Structure") (Hit :type "HitResult Structure (by ref)"))
  (`/Engine/EditorBlueprintResources/StandardMacros.DoOnce` false
    (:`Completed`
      (`self.SERVER_EventHit` HitLocation Hit (`KismetMathLibrary.GetDirectionUnitVector` (`self.K2_GetActorLocation`) (`self.K2_GetActorLocation` Other)) Other self (`self.Damage Type Class`) (`self.Base Damage`)))))

(event `SERVER_EventHit`
  (params (Location :type "Vector Structure") (HitInfo :type "HitResult Structure (by ref)") (HitFromDirection :type "Vector Structure (by ref)") (DamagedActor :type "Actor Object Reference") (DamageCauser :type "Actor Object Reference") (DamageTypeClass :type "DamageType Class Reference") (BaseDamage :type "Float (single-precision)"))
  (`self.CLIENT_EventHit` Location DamageCauser DamageTypeClass HitInfo HitFromDirection DamagedActor BaseDamage))

(event `CLIENT_EventHit`
  (params (Location :type "Vector Structure") (DamageCauser :type "Actor Object Reference") (DamageTypeClass :type "DamageType Class Reference") (HitInfo :type "HitResult Structure (by ref)") (HitFromDirection :type "Vector Structure (by ref)") (DamagedActor :type "Actor Object Reference") (BaseDamage :type "Float (single-precision)"))
  (`GameplayStatics.SpawnEmitterAtLocation` "/Game/VFX/Bonuses/P_BulletImpact_Meat.P_BulletImpact_Meat" Location (struct) (0.4 0.4 0.4))
  (`GameplayStatics.PlaySoundAtLocation` null Location (struct) 1.0 1.0 0.0 null null null null)
  (`GameplayStatics.ApplyPointDamage` DamagedActor BaseDamage HitFromDirection HitInfo null DamageCauser DamageTypeClass)
  (`PrimitiveComponent.SetCollisionEnabled` (`self.Sphere`) "NoCollision")
  (`SceneComponent.SetHiddenInGame` (`self.BulletMesh`) true false)
  (`KismetSystemLibrary.Delay` 0.4)
  (`self.K2_DestroyActor`))

(fn `UserConstructionScript`)