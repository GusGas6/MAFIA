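; Co-op key pickup that bobs and spins on two self-restarting timelines driving the Mover component.
; Sphere overlaps route through server-to-client custom events, which check for BP_ThirdPersonCharacter, tag it "keyholder" and unhide its KeyMesh.
; A DoOnce then waits a tick, spawns impact particles and a sound at the key, and destroys the actor.
; The separate KeyAdd event pair is uncalled here and ends in an empty client event.
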(event `self.ReceiveBeginPlay`
  (`|ExecutionSequence`
    (:`then_0`
      (bind (_direction _newtrack_0) (`Timeline|Timeline` :!via `PlayFromStart` :!label _label)
        (:`Update`
          (`SceneComponent.K2_SetRelativeLocation` (`self.Mover`) (`KismetMathLibrary.VLerp` (0.0 0.0 50.0) (0.0 0.0 75.0) _newtrack_0) false false))
        (:`Finished`
          (`|ExecutionSequence`
            (:`then_0`
              (goto _label :!via `PlayFromStart`))))))
    (:`then_1`
      (bind (_direction_2 _newtrack_0_2) (`Timeline|Timeline_0` :!via `PlayFromStart` :!label _label_2)
        (:`Update`
          (`SceneComponent.K2_SetRelativeRotation` (`self.Mover`) (`KismetMathLibrary.RLerp` (struct) (struct :`Yaw` 360.0) _newtrack_0_2) false false))
        (:`Finished`
          (`|ExecutionSequence`
            (:`then_0`
              (goto _label_2 :!via `PlayFromStart`))))))))

(event `SERVER_KeyAdd`
  (params (Target :type "Actor Object Reference"))
  (`self.CLIENT_KeyAdd` Target))

(event `CLIENT_KeyAdd`
  (params (Target :type "Actor Object Reference")))

(event `CLIENT_OverlapCheck`
  (params (Target :type "Actor Object Reference"))
  (bind _returnvalue (`SceneComponent.K2_GetComponentLocation` (`self.KeyMesh`)))
  (if (== (`GameplayStatics.GetObjectClass` Target) "/Game/Blueprints/BP_ThirdPersonCharacter.BP_ThirdPersonCharacter_C")
    (`|ExecutionSequence`
      (:`then_0`
        (`KismetArrayLibrary.Array_Add` (`Actor.Tags` Target) "keyholder")
        (bind _asbp_third_person_character (cast `/Game/Blueprints/BP_ThirdPersonCharacter` Target))
        (`SceneComponent.SetHiddenInGame` (`/Game/Blueprints/BP_ThirdPersonCharacter.KeyMesh` _asbp_third_person_character) false false))
      (:`then_1`
        (`/Engine/EditorBlueprintResources/StandardMacros.DoOnce` false
          (:`Completed`
            (`KismetSystemLibrary.DelayUntilNextTick`)
            (`GameplayStatics.SpawnEmitterAtLocation` "/Game/VFX/Bonuses/P_BulletImpact.P_BulletImpact" _returnvalue (struct) (0.3 0.3 0.3))
            (`GameplayStatics.SpawnSoundAtLocation` null _returnvalue (struct) 1.0 1.0 0.0 null null)
            (`self.K2_DestroyActor`)))))))

(event `self.Sphere.OnComponentBeginOverlap`
  (params (OverlappedComponent :type "PrimitiveComponent Object Reference") (OtherActor :type "Actor Object Reference") (OtherComp :type "PrimitiveComponent Object Reference") (OtherBodyIndex :type Integer) (bFromSweep :type Boolean) (SweepResult :type "HitResult Structure (by ref)"))
  (`self.SERVER_OverlapCheck` OtherActor))

(event `SERVER_OverlapCheck`
  (params (Target :type "Actor Object Reference"))
  (`self.CLIENT_OverlapCheck` Target))

(fn `UserConstructionScript`)