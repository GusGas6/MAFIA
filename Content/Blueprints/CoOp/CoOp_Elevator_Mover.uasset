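; Co-op elevator that moves a platform between two locations while buttons are held.
; Activate counts holders and plays a normal or FAST timeline; Deactivate reverses it once none remain.
; While deactivated, anything entering the Box takes lethal point damage with gore effect and sound, relayed through server and client events.
; The construction script applies ElevatorSpeed as the actor's CustomTimeDilation to scale movement speed.
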(event `/Game/Blueprints/CoOp/CoOp_BPI.activate`
  (`/Engine/EditorBlueprintResources/StandardMacros.IncrementInt` (`self.AmountOfButtonsHolding`)
    (:`  `
      (set `self.Deactivated` false)
      (if (`self.FAST`)
        (bind (_direction _newtrack_0) (`Timeline|Timeline_0` :!label _label)
          (:`Update`
            (`SceneComponent.K2_SetRelativeLocation` (`self.PlatformMesh`) (`KismetMathLibrary.VLerp` (`self.ElevatorLocation1`) (`self.ElevatorLocation2`) _newtrack_0) false false)))
        (else
          (bind (_direction_2 _newtrack_0_2) (`Timeline|Timeline` :!label _label_2)
            (:`Update`
              (`SceneComponent.K2_SetRelativeLocation` (`self.PlatformMesh`) (`KismetMathLibrary.VLerp` (`self.ElevatorLocation1`) (`self.ElevatorLocation2`) _newtrack_0_2) false false))))))))

(event `/Game/Blueprints/CoOp/CoOp_BPI.deactivate`
  (bind _amountofbuttonsholding (`self.AmountOfButtonsHolding`))
  (`/Engine/EditorBlueprintResources/StandardMacros.DecrementInt` _amountofbuttonsholding
    (:`  `
      (if (<= _amountofbuttonsholding 0)
        (set `self.Deactivated` true)
        (if (`self.FAST`)
          (goto _label :!via `Reverse`)
          (else
            (goto _label_2 :!via `Reverse`)))))))

(event `self.Box.OnComponentBeginOverlap`
  (params (OverlappedComponent :type "PrimitiveComponent Object Reference") (OtherActor :type "Actor Object Reference") (OtherComp :type "PrimitiveComponent Object Reference") (OtherBodyIndex :type Integer) (bFromSweep :type Boolean) (SweepResult :type "HitResult Structure (by ref)"))
  (if (`self.Deactivated`)
    (`self.SERVER_ElevatorCrush` OtherActor 999.0 (`KismetMathLibrary.GetDirectionUnitVector` (`self.K2_GetActorLocation`) (`self.K2_GetActorLocation` OtherActor)) SweepResult self)))

(event `SERVER_ElevatorCrush`
  (params (DamagedActor :type "Actor Object Reference") (BaseDamage :type "Float (single-precision)") (HitFromDirection :type "Vector Structure (by ref)") (HitInfo :type "HitResult Structure (by ref)") (DamageCauser :type "Actor Object Reference") (DamageTypeClass :type "DamageType Class Reference"))
  (`self.CLIENT_ElevatorCrush` DamagedActor BaseDamage HitFromDirection HitInfo DamageCauser DamageTypeClass))

(event `CLIENT_ElevatorCrush`
  (params (DamagedActor :type "Actor Object Reference") (BaseDamage :type "Float (single-precision)") (HitFromDirection :type "Vector Structure (by ref)") (HitInfo :type "HitResult Structure (by ref)") (DamageCauser :type "Actor Object Reference") (DamageTypeClass :type "DamageType Class Reference"))
  (bind (_bblockinghit _binitialoverlap _time _distance _location) (`GameplayStatics.BreakHitResult` HitInfo))
  (`GameplayStatics.ApplyPointDamage` DamagedActor BaseDamage HitFromDirection HitInfo null DamageCauser DamageTypeClass)
  (`GameplayStatics.SpawnEmitterAtLocation` "/Game/VFX/Bonuses/P_BulletImpact_Meat.P_BulletImpact_Meat" _location)
  (`GameplayStatics.PlaySoundAtLocation` null _location (struct) 1.0 1.0 0.0 null null null null))

(fn `UserConstructionScript`
  (set `self.CustomTimeDilation` (`self.ElevatorSpeed`)))