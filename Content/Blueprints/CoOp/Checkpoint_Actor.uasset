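; Co-op checkpoint airlock that needs a keyholder to unlock and every networked player present to save.
; The lock overlap consumes the key, animates it, bursts the lock with physics gibs, then slowly opens the entrance doors.
; Once all players fill the box, it stores their checkpoint locations, activates nearby enemy spawners, opens exit doors and closes entrance doors.
; Overlaps and timeline-driven doors relay through Server-to-Client events, with polled text showing the player count.
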(event `self.ReceiveBeginPlay`
  (`KismetArrayLibrary.Array_Append` (`self.ActorsToActivate`) (`PrimitiveComponent.GetOverlappingActors` (`self.ActorsToRespawnBox`) "/Game/Blueprints/AI/EnemySpawner_BP.EnemySpawner_BP_C")))

(event `/Game/Blueprints/CoOp/CoOp_BPI.activate`
  (for _array_element (`self.ActorsToActivate`) :!label _label
    (message `/Game/Blueprints/CoOp/CoOp_BPI.activate` _array_element)))

(event `CLIENT_OverlapCheck`
  (params (Target :type "Actor Object Reference"))
  (bind _numnetplayers (`AdvancedSessionsLibrary.GetNumberOfNetworkPlayers`))
  (bind _textrender (`self.TextRender`))
  (bind _returnvalue (`KismetArrayLibrary.Array_Length` (`PrimitiveComponent.GetOverlappingActors` (`self.Box`) "/Game/Blueprints/BP_ThirdPersonCharacter.BP_ThirdPersonCharacter_C")))
  (if (== (`GameplayStatics.GetObjectClass` Target) "/Game/Blueprints/BP_ThirdPersonCharacter.BP_ThirdPersonCharacter_C")
    (if (`self.ActorHasTag` Target "keyholder")
      (bind _asbp_third_person_character (cast `/Game/Blueprints/BP_ThirdPersonCharacter` Target))
      (`KismetArrayLibrary.Array_RemoveItem` (`Actor.Tags` _asbp_third_person_character) "keyholder")
      (`SceneComponent.SetHiddenInGame` (`/Game/Blueprints/BP_ThirdPersonCharacter.KeyMesh` _asbp_third_person_character) true false)
      (set `self.KeyProvided` true)
      (if (== _returnvalue _numnetplayers) :!label _label_2
        (`/Engine/EditorBlueprintResources/StandardMacros.DoOnce` false
          (:`Completed`
            (bind _outactors (`GameplayStatics.GetAllActorsOfClass` "/Game/Blueprints/BP_ThirdPersonCharacter.BP_ThirdPersonCharacter_C"))
            (for _array_element _outactors
              (`/Game/Blueprints/BP_ThirdPersonCharacter.SERVER_StoreCheckpointLocation` _array_element (`self.K2_GetActorLocation` _array_element) self)
              (`KismetSystemLibrary.PrintString` "CHECKPOINT SUCCESS")
              (`SceneComponent.SetHiddenInGame` (`self.TextRender`) true false)
              (set `self.CheckpointSaved` true)
              (goto _label))
            (`self.SERVER_ActivateExitDoors` false)
            (`self.SERVER_ActivateEntranceDoors` true)))
        (else
          (`KismetSystemLibrary.PrintString` "WAITING FOR OTHER PLAYERS TO ARRIVE..." true true (struct :`R` 0.75141 :`G` 0.063935 :`B` 1.0 :`A` 1.0))
          (`SceneComponent.SetHiddenInGame` _textrender false false)
          (`TextRenderComponent.K2_SetText` _textrender (`KismetTextLibrary.Conv_StringToText` (`KismetStringLibrary.Concat_StrStr` (`KismetStringLibrary.Conv_IntToString` _returnvalue) " / " (`KismetStringLibrary.Conv_IntToString` _numnetplayers) " PLAYERS")) :!label _label_3)
          (if (not (`self.CheckpointSaved`))
            (`KismetSystemLibrary.Delay` 0.1)
            (goto _label_3))))
      (elif (`self.KeyProvided`)
        (goto _label_2)
        (else
          (`KismetSystemLibrary.PrintString` "NO KEY" true true (struct :`R` 1.0 :`B` 0.038846 :`A` 1.0)))))))

(event `self.Box.OnComponentBeginOverlap`
  (params (OverlappedComponent :type "PrimitiveComponent Object Reference") (OtherActor :type "Actor Object Reference") (OtherComp :type "PrimitiveComponent Object Reference") (OtherBodyIndex :type Integer) (bFromSweep :type Boolean) (SweepResult :type "HitResult Structure (by ref)"))
  (`self.SERVER_OverlapCheck` OtherActor))

(event `SERVER_OverlapCheck`
  (params (Target :type "Actor Object Reference"))
  (`self.CLIENT_OverlapCheck` Target))

(event `self.LockOverlapBox.OnComponentBeginOverlap`
  (params (OverlappedComponent :type "PrimitiveComponent Object Reference") (OtherActor :type "Actor Object Reference") (OtherComp :type "PrimitiveComponent Object Reference") (OtherBodyIndex :type Integer) (bFromSweep :type Boolean) (SweepResult :type "HitResult Structure (by ref)"))
  (`self.SERVER_LockOverlapCheck` OtherActor))

(event `SERVER_LockOverlapCheck`
  (params (Target :type "Actor Object Reference"))
  (`self.CLIENT_LockOverlapCheck` Target))

(event `CLIENT_LockOverlapCheck`
  (params (Target :type "Actor Object Reference"))
  (bind _sm_bulkheadlock (`self.SM_BulkheadLock`))
  (bind _sm_bulkheadgibbottom (`self.SM_BulkheadGibBottom`))
  (bind _returnvalue (`SceneComponent.K2_GetComponentLocation` _sm_bulkheadlock))
  (if (`self.ActorHasTag` Target "keyholder")
    (bind _asbp_third_person_character (cast `/Game/Blueprints/BP_ThirdPersonCharacter` Target))
    (`KismetArrayLibrary.Array_RemoveItem` (`Actor.Tags` _asbp_third_person_character) "keyholder")
    (`SceneComponent.SetHiddenInGame` (`/Game/Blueprints/BP_ThirdPersonCharacter.KeyMesh` _asbp_third_person_character) true false)
    (set `self.KeyProvided` true)
    (`SceneComponent.SetHiddenInGame` (`self.Key`) false false)
    (bind (_direction _newtrack_0) (`Timeline|Timeline_2` :!via `PlayFromStart`)
      (:`Update`
        (`SceneComponent.K2_SetRelativeLocation` (`self.Key`) (`KismetMathLibrary.VLerp` (-150.0 0.0 0.0) (-85.0 0.0 0.0) _newtrack_0) false false))
      (:`Finished`
        (`KismetSystemLibrary.Delay` 0.2)
        (bind (_direction_2 _newtrack_0_2) (`Timeline|Timeline_3` :!via `PlayFromStart`)
          (:`Update`
            (`SceneComponent.K2_SetRelativeRotation` (`self.Key`) (`KismetMathLibrary.RLerp` (struct) (struct :`Roll` 180.0) _newtrack_0_2) false false))
          (:`Finished`
            (`GameplayStatics.SpawnEmitterAtLocation` "/Game/VFX/Bonuses/P_Refraction.P_Refraction" _returnvalue)
            (`GameplayStatics.SpawnSoundAtLocation` null _returnvalue (struct) 1.0 1.0 0.0 null null)
            (`ActorComponent.K2_DestroyComponent` _sm_bulkheadlock)
            (`ActorComponent.K2_DestroyComponent` (`self.Key`))
            (`PrimitiveComponent.SetSimulatePhysics` _sm_bulkheadgibbottom true)
            (`PrimitiveComponent.SetSimulatePhysics` (`self.SM_BulkheadGibTop`) true)
            (bind _returnvalue_2 (* (`KismetMathLibrary.RandomUnitVectorInConeInDegrees` (`self.GetActorForwardVector` _asbp_third_person_character) 35.0) (`KismetMathLibrary.RandomFloatInRange` 300.0 600.0)))
            (`PrimitiveComponent.AddImpulse` _sm_bulkheadgibbottom _returnvalue_2 "None" true)
            (`PrimitiveComponent.AddImpulse` (`self.SM_BulkheadGibTop`) _returnvalue_2 "None" true)
            (`KismetSystemLibrary.Delay` 1.0)
            (`self.SERVER_ActivateEntranceDoors` false true)))))
    (elif (not (`self.KeyProvided`))
      (`KismetSystemLibrary.PrintString` "NO KEY" true true (struct :`R` 1.0 :`B` 0.038846 :`A` 1.0)))))

(event `SERVER_ActivateEntranceDoors`
  (params (Reverse :type Boolean) (Slow :type Boolean))
  (`self.CLIENT_ActivateEntranceDoors` Reverse Slow))

(event `CLIENT_ActivateEntranceDoors`
  (params (Reverse :type Boolean) (Slow :type Boolean))
  (if Slow
    (bind (_direction _newtrack_1) (`Timeline|Timeline_1` :!via `PlayFromStart` :!label _label_4)
      (:`Update`
        (`SceneComponent.K2_SetRelativeLocation` (`self.BulkheadDoorsEntrance`) (`KismetMathLibrary.VLerp` (166.52674 -319.338298 1e-06) (426.743623 -319.338298 1e-06) _newtrack_1) false false)
        (`SceneComponent.K2_SetRelativeLocation` (`self.BulkheadDoorsEntrance1`) (`KismetMathLibrary.VLerp` (-182.742124 -319.338289 3e-06) (-438.26068 -319.338289 3e-06) _newtrack_1) false false)))
    (else
      (`|ExecutionSequence`
        (:`then_0`
          (goto _label_4 :!via `Stop`))
        (:`then_1`
          (`KismetSystemLibrary.DelayUntilNextTick`)
          (if Reverse
            (bind (_direction_2 _newtrack_1_2) (`Timeline|Timeline` :!via `Reverse` :!label _label_5)
              (:`Update`
                (`SceneComponent.K2_SetRelativeLocation` (`self.BulkheadDoorsEntrance`) (`KismetMathLibrary.VLerp` (166.52674 -319.338298 1e-06) (426.743623 -319.338298 1e-06) _newtrack_1_2) false false)
                (`SceneComponent.K2_SetRelativeLocation` (`self.BulkheadDoorsEntrance1`) (`KismetMathLibrary.VLerp` (-182.742124 -319.338289 3e-06) (-438.26068 -319.338289 3e-06) _newtrack_1_2) false false)))
            (else
              (goto _label_5))))))))

(event `SERVER_ActivateExitDoors`
  (params (Reverse :type Boolean))
  (`self.CLIENT_ActivateExitDoors` Reverse))

(event `CLIENT_ActivateExitDoors`
  (params (Reverse :type Boolean))
  (if Reverse
    (bind (_direction _newtrack_1) (`Timeline|Timeline_0` :!via `Reverse` :!label _label_6)
      (:`Update`
        (`SceneComponent.K2_SetRelativeLocation` (`self.BulkheadDoorsExit`) (`KismetMathLibrary.VLerp` (-184.478521 303.099516 1e-06) (-435.561606 303.099516 1e-06) _newtrack_1) false false)
        (`SceneComponent.K2_SetRelativeLocation` (`self.BulkheadDoorsExit1`) (`KismetMathLibrary.VLerp` (166.52675 303.099507 1e-06) (421.760576 303.099507 1e-06) _newtrack_1) false false)))
    (else
      (goto _label_6))))

(fn `UserConstructionScript`)