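; Co-op extraction helicopter that serves as the win point, with two rotor blades spun by a self-restarting Timeline.
; Box overlaps pass through server and client check events, comparing overlapping characters to the network player count.
; When all players are inside, a DoOnce shows the win screen on every character's HUD; otherwise a text render reveals a looping arrived-player count.
; An unconnected chain would destroy the session and open the main menu.
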(event `self.ReceiveBeginPlay`
  (bind (_direction _newtrack_0) (`Timeline|Timeline` :!via `PlayFromStart` :!label _label)
    (:`Update`
      (`SceneComponent.K2_SetRelativeRotation` (`self.SM_HelicopterBlade`) (`KismetMathLibrary.RLerp` (struct) (struct :`Yaw` 360.0) _newtrack_0) false false)
      (`SceneComponent.K2_SetRelativeRotation` (`self.SM_HelicopterBlade1`) (`KismetMathLibrary.RLerp` (struct :`Roll` -20.0) (struct :`Yaw` -360.0 :`Roll` -20.0) _newtrack_0) false false))
    (:`Finished`
      (`|ExecutionSequence`
        (:`then_0`
          (goto _label :!via `PlayFromStart`))))))

(event `CLIENT_OverlapCheck`
  (params (Target :type "Actor Object Reference") (Target2 :type "PrimitiveComponent Object Reference") (Target3 :type "SceneComponent Object Reference") (Target4 :type "TextRenderComponent Object Reference"))
  (bind _numnetplayers (`AdvancedSessionsLibrary.GetNumberOfNetworkPlayers`))
  (bind _returnvalue (`KismetArrayLibrary.Array_Length` (`PrimitiveComponent.GetOverlappingActors` Target2 "/Game/Blueprints/BP_ThirdPersonCharacter.BP_ThirdPersonCharacter_C")))
  (if (== (`GameplayStatics.GetObjectClass` Target) "/Game/Blueprints/BP_ThirdPersonCharacter.BP_ThirdPersonCharacter_C")
    (if (== _returnvalue _numnetplayers)
      (`/Engine/EditorBlueprintResources/StandardMacros.DoOnce` false
        (:`Completed`
          (bind _outactors (`GameplayStatics.GetAllActorsOfClass` "/Game/Blueprints/BP_ThirdPersonCharacter.BP_ThirdPersonCharacter_C"))
          (for _array_element _outactors
            (`/Game/UI/PlayerHUD_WBP.YOUWIN` (`/Game/Blueprints/BP_ThirdPersonCharacter.PlayerHUD` _array_element)))))
      (else
        (`KismetSystemLibrary.PrintString` "WAITING FOR OTHER PLAYERS TO ARRIVE..." true true (struct :`R` 0.75141 :`G` 0.063935 :`B` 1.0 :`A` 1.0))
        (`SceneComponent.SetHiddenInGame` Target3 false false)
        (`TextRenderComponent.K2_SetText` Target4 (`KismetTextLibrary.Conv_StringToText` (`KismetStringLibrary.Concat_StrStr` (`KismetStringLibrary.Conv_IntToString` _returnvalue) " / " (`KismetStringLibrary.Conv_IntToString` _numnetplayers) " PLAYERS")) :!label _label_2)
        (`KismetSystemLibrary.Delay` 0.1)
        (goto _label_2)))))

(event `self.Box.OnComponentBeginOverlap`
  (params (OverlappedComponent :type "PrimitiveComponent Object Reference") (OtherActor :type "Actor Object Reference") (OtherComp :type "PrimitiveComponent Object Reference") (OtherBodyIndex :type Integer) (bFromSweep :type Boolean) (SweepResult :type "HitResult Structure (by ref)"))
  (bind _textrender (`self.TextRender`))
  (`self.SERVER_OverlapCheck` OtherActor (`self.Box`) _textrender _textrender))

(event `SERVER_OverlapCheck`
  (params (Target :type "Actor Object Reference") (Target2 :type "PrimitiveComponent Object Reference") (Target3 :type "SceneComponent Object Reference") (Target4 :type "TextRenderComponent Object Reference"))
  (`self.CLIENT_OverlapCheck` Target Target2 Target3 Target4))

(fn `UserConstructionScript`)