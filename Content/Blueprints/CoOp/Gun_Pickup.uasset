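; Co-op weapon pickup that gives an overlapping third-person character a revolver, shotgun or tommy gun, as chosen per instance.
; The construction script sets the mesh and label, while two looping timelines bob and spin it.
; Overlap passes through server-then-client events to equip the weapon and play effects.
; The pickup then becomes the player's previous weapon, without updating its label, or destroys itself if there was none.
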(event `self.ReceiveBeginPlay`
  (`|ExecutionSequence`
    (:`then_0`
      (bind (_direction _newtrack_0) (`Timeline|Timeline` :!via `PlayFromStart` :!label _label)
        (:`Update`
          (`SceneComponent.K2_SetRelativeLocation` (`self.Mover`) (`KismetMathLibrary.VLerp` (0.0 0.0 50.0) (0.0 0.0 75.0) _newtrack_0) false false))
        (:`Finished`
          (`|ExecutionSequence`
            (:`then_0`
              (goto _label :!via `PlayFromStart`))))))
    (:`then_1`
      (bind (_direction_2 _newtrack_0_2) (`Timeline|Timeline_0` :!via `PlayFromStart` :!label _label_2)
        (:`Update`
          (`SceneComponent.K2_SetRelativeRotation` (`self.Mover`) (`KismetMathLibrary.RLerp` (struct) (struct :`Yaw` 360.0) _newtrack_0_2) false false))
        (:`Finished`
          (`|ExecutionSequence`
            (:`then_0`
              (goto _label_2 :!via `PlayFromStart`))))))))

(event `CLIENT_OverlapCheck`
  (params (Target :type "Actor Object Reference"))
  (bind _gunmesh (`self.GunMesh`))
  (bind _storepreviousplayerweapon (`self.StorePreviousPlayerWeapon`))
  (bind _returnvalue (`SceneComponent.K2_GetComponentLocation` (`self.GunMesh`)))
  (if (== (`GameplayStatics.GetObjectClass` Target) "/Game/Blueprints/BP_ThirdPersonCharacter.BP_ThirdPersonCharacter_C")
    (`|ExecutionSequence`
      (:`then_0`
        (bind _asbp_third_person_character (cast `/Game/Blueprints/BP_ThirdPersonCharacter` Target))
        (set `self.StorePreviousPlayerWeapon` (`/Game/Blueprints/BP_ThirdPersonCharacter.EquippedWeapon` _asbp_third_person_character))
        (`/Game/Blueprints/BP_ThirdPersonCharacter.SERVER_EquipWeapon` _asbp_third_person_character (`self.WeaponName`)))
      (:`then_1`
        (`KismetSystemLibrary.DelayUntilNextTick`)
        (`GameplayStatics.SpawnEmitterAtLocation` "/Game/VFX/Bonuses/P_MuzzleFlashBasic.P_MuzzleFlashBasic" _returnvalue (struct) (0.1 0.1 0.1))
        (`GameplayStatics.SpawnSoundAtLocation` null _returnvalue (struct) 1.0 1.0 0.0 null null)
        (if (== _storepreviousplayerweapon "None")
          (`self.K2_DestroyActor`)
          (else
            (switch `name` _storepreviousplayerweapon
              (:`revolver`
                (set `self.WeaponName` "Revolver")
                (`StaticMeshComponent.SetStaticMesh` _gunmesh "/Game/Models/Blockouts/SM_Pistol.SM_Pistol"))
              (:`shotgun`
                (set `self.WeaponName` "Shotgun")
                (`StaticMeshComponent.SetStaticMesh` _gunmesh "/Game/Models/Blockouts/SM_Shotgun.SM_Shotgun"))
              (:`tommygun`
                (set `self.WeaponName` "Tommygun")
                (`StaticMeshComponent.SetStaticMesh` _gunmesh "/Game/Models/Blockouts/SM_Tommygun.SM_Tommygun")))))))))

(event `self.Sphere.OnComponentBeginOverlap`
  (params (OverlappedComponent :type "PrimitiveComponent Object Reference") (OtherActor :type "Actor Object Reference") (OtherComp :type "PrimitiveComponent Object Reference") (OtherBodyIndex :type Integer) (bFromSweep :type Boolean) (SweepResult :type "HitResult Structure (by ref)"))
  (`self.SERVER_OverlapCheck` OtherActor))

(event `SERVER_OverlapCheck`
  (params (Target :type "Actor Object Reference"))
  (`self.CLIENT_OverlapCheck` Target))

(fn `UserConstructionScript`
  (bind _gunmesh (`self.GunMesh`))
  (switch `/Game/Blueprints/CoOp/WeaponTypes_Enum` (`self.Weapons`)
    (:`NewEnumerator0`
      (set `self.WeaponName` "Revolver")
      (`StaticMeshComponent.SetStaticMesh` _gunmesh "/Game/Models/Blockouts/SM_Pistol.SM_Pistol"))
    (:`NewEnumerator1`
      (set `self.WeaponName` "Shotgun")
      (`StaticMeshComponent.SetStaticMesh` _gunmesh "/Game/Models/Blockouts/SM_Shotgun.SM_Shotgun"))
    (:`NewEnumerator2`
      (set `self.WeaponName` "Tommygun")
      (`StaticMeshComponent.SetStaticMesh` _gunmesh "/Game/Models/Blockouts/SM_Tommygun.SM_Tommygun")))
  (`TextRenderComponent.K2_SetText` (`self.TextRender`) (`KismetTextLibrary.Conv_NameToText` (`self.WeaponName`))))