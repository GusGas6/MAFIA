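; Co-op pressure-switch trigger that activates linked elevators while a third-person character overlaps it, warning on BeginPlay if none are linked.
; Overlap begin and end pass through SERVER events to CLIENT events, which send activate or deactivate messages to every linked elevator.
; The same events play or reverse a timeline that sinks the sphere slightly and raises it again.
; End overlap deactivates without checking for remaining occupants.
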(event `self.ReceiveBeginPlay`
  (if (== (`KismetArrayLibrary.Array_Length` (`self.LinkedElevators`)) 0)
    (`KismetSystemLibrary.PrintString` (`KismetStringLibrary.Concat_StrStr` "WARNING!! " (`KismetSystemLibrary.GetDisplayName` self) " HAS NO DESIGNATED THING TO ACTIVATE") true true (struct :`R` 1.0 :`B` 0.031279 :`A` 1.0))))

(event `self.ActivateElevator.OnComponentBeginOverlap`
  (params (OverlappedComponent :type "PrimitiveComponent Object Reference") (OtherActor :type "Actor Object Reference") (OtherComp :type "PrimitiveComponent Object Reference") (OtherBodyIndex :type Integer) (bFromSweep :type Boolean) (SweepResult :type "HitResult Structure (by ref)"))
  (if (== (`GameplayStatics.GetObjectClass` OtherActor) "/Game/ThirdPerson/Blueprints/BP_ThirdPersonCharacter.BP_ThirdPersonCharacter_C")
    (`self.SERVER_Overlap`)))

(event `SERVER_Overlap`
  (`self.CLIENT_Overlap`))

(event `CLIENT_Overlap`
  (for _array_element (`self.LinkedElevators`)
    (message `/Game/Blueprints/CoOp/CoOp_BPI.activate` _array_element))
  (bind (_direction _newtrack_0) (`Timeline|Timeline` :!label _label)
    (:`Update`
      (`SceneComponent.K2_SetRelativeLocation` (`self.Sphere`) (`KismetMathLibrary.VLerp` (0.0 0.0 0.0) (0.0 0.0 -7.0) _newtrack_0) false false))))

(event `self.ActivateElevator.OnComponentEndOverlap`
  (params (OverlappedComponent :type "PrimitiveComponent Object Reference") (OtherActor :type "Actor Object Reference") (OtherComp :type "PrimitiveComponent Object Reference") (OtherBodyIndex :type Integer))
  (if (== (`GameplayStatics.GetObjectClass` OtherActor) "/Game/ThirdPerson/Blueprints/BP_ThirdPersonCharacter.BP_ThirdPersonCharacter_C")
    (`self.SERVER_EndOverlap`)))

(event `SERVER_EndOverlap`
  (`self.CLIENT_EndOverlap`))

(event `CLIENT_EndOverlap`
  (for _array_element (`self.LinkedElevators`)
    (message `/Game/Blueprints/CoOp/CoOp_BPI.deactivate` _array_element))
  (goto _label :!via `Reverse`))

(fn `UserConstructionScript`)