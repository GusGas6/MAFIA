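; Rotating warning light with an alarm, switched on and off through StartSpinning and StopSpinning.
; A self-restarting timeline yaws the Mover component through full turns while two rect lights are visible.
; A DoOnce-gated delay loop reactivates Alarm periodically while Spinning; stopping hides the lights and resets the gate.
; With EndRoomLights set, it starts spinning on BeginPlay as a dim green light.
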(event `self.ReceiveBeginPlay`
  (if (`self.EndRoomLights`)
    (`self.StartSpinning`)
    (`LightComponent.SetLightColor` (`self.RectLight1`) (struct :`R` 0.009315 :`G` 0.5625 :`A` 1.0) true)
    (`LightComponent.SetLightColor` (`self.RectLight`) (struct :`R` 0.009315 :`G` 0.5625 :`A` 1.0) true)
    (`LightComponent.SetIntensity` (`self.RectLight`) 0.2)
    (`LightComponent.SetIntensity` (`self.RectLight1`) 0.2)))

(event `StartSpinning`
  (set `self.Spinning` true)
  (`|ExecutionSequence`
    (:`then_0`
      (`SceneComponent.SetVisibility` (`self.RectLight`) true false)
      (`SceneComponent.SetVisibility` (`self.RectLight1`) true false)
      (bind (_direction _newtrack_0) (`Timeline|Timeline` :!label _label)
        (:`Update`
          (`SceneComponent.K2_SetRelativeRotation` (`self.Mover`) (`KismetMathLibrary.RLerp` (struct) (struct :`Pitch` 360.0) _newtrack_0) false false))
        (:`Finished`
          (`|ExecutionSequence`
            (:`then_0`
              (goto _label :!via `PlayFromStart`))))))
    (:`then_1`
      (`/Engine/EditorBlueprintResources/StandardMacros.DoOnce` false :!label _label_2
        (:`Completed`
          (if (`self.Spinning`) :!label _label_3
            (`ActorComponent.Activate` (`self.Alarm`) true)
            (`KismetSystemLibrary.Delay` 30.0)
            (goto _label_3)))))))

(event `StopSpinning`
  (`|ExecutionSequence`
    (:`then_0`
      (set `self.Spinning` false)
      (`SceneComponent.SetVisibility` (`self.RectLight`) false false)
      (`SceneComponent.SetVisibility` (`self.RectLight1`) false false)
      (goto _label :!via `Stop`))
    (:`then_1`
      (goto _label_2 :!via `Reset`))))

(fn `UserConstructionScript`)